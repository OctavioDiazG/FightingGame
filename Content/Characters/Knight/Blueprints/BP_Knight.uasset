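; BP_Knight is the Knight character in a two-player game, defining only its Special attack.
; The Special event picks the opponent from IsPlayer2 and compares both players' X positions to decide which way to attack.
; It spawns a BP_Special slightly offset toward the opponent, passing the Knight and opponent references, with a negative Direction for leftward attacks and the default otherwise.
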(event `Special`
  (bind _returnvalue_x (`KismetMathLibrary.BreakVector` (`self.K2_GetActorLocation` (`self.player1`))))
  (bind _returnvalue_x_2 (`KismetMathLibrary.BreakVector` (`self.K2_GetActorLocation` (`self.player2`))))
  (bind _returnvalue_x_3 (`KismetMathLibrary.BreakVector` (`self.K2_GetActorLocation` (`self.player2`))))
  (bind _returnvalue_x_4 (`KismetMathLibrary.BreakVector` (`self.K2_GetActorLocation` (`self.player1`))))
  (if (`self.isPlayer2`)
    (if (> _returnvalue_x_3 _returnvalue_x_4)
      (`|SpawnActorFromClass` "/Game/Characters/Knight/Blueprints/BP_Special.BP_Special_C" (`KismetMathLibrary.MakeTransform` (+ (`self.K2_GetActorLocation`) (-100.0 0.0 0.0)) (`self.K2_GetActorRotation`)) "AlwaysSpawn" "MultiplyWithRoot" null self (`self.player1`) -10.0 null)
      (else
        (`|SpawnActorFromClass` "/Game/Characters/Knight/Blueprints/BP_Special.BP_Special_C" (`KismetMathLibrary.MakeTransform` (+ (`self.K2_GetActorLocation`) (100.0 0.0 0.0)) (`self.K2_GetActorRotation`)) "AlwaysSpawn" "MultiplyWithRoot" null self (`self.player1`) 10.0 null)))
    (elif (> _returnvalue_x _returnvalue_x_2)
      (`|SpawnActorFromClass` "/Game/Characters/Knight/Blueprints/BP_Special.BP_Special_C" (`KismetMathLibrary.MakeTransform` (+ (`self.K2_GetActorLocation`) (-100.0 0.0 0.0)) (`self.K2_GetActorRotation`)) "AlwaysSpawn" "MultiplyWithRoot" null self (`self.player2`) -10.0 null)
      (else
        (`|SpawnActorFromClass` "/Game/Characters/Knight/Blueprints/BP_Special.BP_Special_C" (`KismetMathLibrary.MakeTransform` (+ (`self.K2_GetActorLocation`) (100.0 0.0 0.0)) (`self.K2_GetActorRotation`)) "AlwaysSpawn" "MultiplyWithRoot" null self (`self.player2`) 10.0 null)))))

(fn `UserConstructionScript`
  (`parent.UserConstructionScript`))