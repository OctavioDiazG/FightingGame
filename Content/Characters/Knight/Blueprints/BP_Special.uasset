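; BP_Special is the Knight's special attack actor: a Paper2D flipbook that travels along X and deals damage.
; A timeline moves the flipbook by a Lerp from its current X toward an offset of Direction on each update.
; The same update polls the Box's overlapping actors, skips the owning Knight, and applies damage through a DoOnce, so only one hit lands.
; A timer destroys the actor after a fixed lifetime.
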(event `self.ReceiveBeginPlay`
  (bind _paperflipbook (`self.PaperFlipbook`))
  (bind (_returnvalue_x _returnvalue_y _returnvalue_z) (`KismetMathLibrary.BreakVector` (`SceneComponent.K2_GetComponentLocation` _paperflipbook)))
  (`KismetSystemLibrary.K2_SetTimerDelegate` (delegate `Destroy`) 7.0)
  (bind (_direction _alpha) (`Timeline|Timeline` :!via `PlayFromStart`)
    (:`Update`
      (`SceneComponent.K2_SetWorldLocation` _paperflipbook (`KismetMathLibrary.MakeVector` (`KismetMathLibrary.Lerp` _returnvalue_x (+ _returnvalue_x (`self.Direction`)) _alpha) _returnvalue_y _returnvalue_z) false false)
      (for _array_element (`PrimitiveComponent.GetOverlappingActors` (`self.Box`) null)
        (if (!= _array_element (`self.As BP Knight`))
          (`/Engine/EditorBlueprintResources/StandardMacros.DoOnce` false
            (:`Completed`
              (`GameplayStatics.ApplyDamage` _array_element 0.75))))))))

(event `Destroy`
  (`self.K2_DestroyActor`))

(event `self.ReceiveTick`
  (params (DeltaSeconds :type "Float (single-precision)")))

(event `self.Box.OnComponentHit`
  (params (HitComponent :type "PrimitiveComponent Object Reference") (OtherActor :type "Actor Object Reference") (OtherComp :type "PrimitiveComponent Object Reference") (NormalImpulse :type "Vector Structure") (Hit :type "HitResult Structure (by ref)")))

(fn `UserConstructionScript`)